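; Trigger volume that switches the player's camera when the third-person character enters it.
; On overlap, it finds the first actor of the class selected from its ActorClass array by ConnectedCam.
; It stores that actor as the character's Currentcam and makes it the player controller's view target via SetViewTargetWithBlend.
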(event `self.OverlapVolume.OnComponentBeginOverlap`
  (params (OverlappedComponent :type "PrimitiveComponent Object Reference") (OtherActor :type "Actor Object Reference") (OtherComp :type "PrimitiveComponent Object Reference") (OtherBodyIndex :type Integer) (bFromSweep :type Boolean) (SweepResult :type "HitResult Structure (by ref)"))
  (bind _asbp_third_person_character (cast `/Game/Dynamic/ThirdPerson/Blueprints/BP_ThirdPersonCharacter` OtherActor))
  (if (`KismetSystemLibrary.IsValid` _asbp_third_person_character)
    (bind _asplayer_controller (cast `PlayerController` (`Pawn.GetController` _asbp_third_person_character)))
    (if (`KismetSystemLibrary.IsValid` _asplayer_controller)
      (bind _returnvalue (`GameplayStatics.GetActorOfClass` (`|GetArrayItem` (`self.ActorClass`) (`self.ConnectedCam`))))
      (bind _output_get (set `/Game/Dynamic/ThirdPerson/Blueprints/BP_ThirdPersonCharacter.Currentcam` _returnvalue _asbp_third_person_character))
      (`PlayerController.SetViewTargetWithBlend` _asplayer_controller _output_get 0.0 "VTBlend_Linear" 0.0 false))))

(fn `UserConstructionScript`)