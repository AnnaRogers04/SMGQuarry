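; BP_FixedCam plays an opening UI sequence while the player character's input is disabled; its graphs contain no camera logic despite the name.
; On BeginPlay it casts the player pawn to BP_ThirdPersonCharacter, disables its input, then adds an OpeningScene widget to the viewport and plays its OPENING animation.
; A Delay fed by the play length queried from PlayAnimation's result times when input is re-enabled.
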(event `self.ReceiveBeginPlay`
  (bind _asbp_third_person_character (cast `/Game/Dynamic/ThirdPerson/Blueprints/BP_ThirdPersonCharacter` (`GameplayStatics.GetPlayerCharacter` 0)))
  (bind _output_get (set `self.As BP Third Person Character` _asbp_third_person_character))
  (`self.DisableInput` _output_get null)
  (bind _returnvalue (`|CreateWidget` "/Game/Dynamic/Interact/UI_Widgets/OpeningScene.OpeningScene_C" (`GameplayStatics.GetPlayerController` 0)))
  (`UserWidget.AddToViewport` _returnvalue 0)
  (bind _returnvalue_2 (`UserWidget.PlayAnimation` _returnvalue (`/Game/Dynamic/Interact/UI_Widgets/OpeningScene.OPENING` _returnvalue) 0.0 1 "Forward" 1.0 false))
  (bind _returnvalue_3 (message `AnimationDataModel.GetPlayLength` _returnvalue_2))
  (`KismetSystemLibrary.Delay` _returnvalue_3)
  (`self.EnableInput` (`self.As BP Third Person Character`) null))

(fn `UserConstructionScript`)