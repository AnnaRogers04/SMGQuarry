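; BP_FixedCam9Pan is a fixed camera that pans back and forth continuously by rotating around its yaw axis.
; On BeginPlay, the Pan timeline adds its track value to the camera component's initial world yaw, keeping roll and pitch.
; When the timeline finishes, Reset waits briefly, then a FlipFlop alternates between reversing and playing it, creating an endless sweep with short pauses at each end.
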(event `self.ReceiveBeginPlay`
  (bind (_returnvalue_roll _returnvalue_pitch _returnvalue_yaw) (`KismetMathLibrary.BreakRotator` (`SceneComponent.K2_GetComponentRotation` (`self.CameraComponent`))))
  (set `self.Return Value X (Roll)` _returnvalue_roll)
  (set `self.Return Value Y (Pitch)` _returnvalue_pitch)
  (set `self.Return Value Z (Yaw)` _returnvalue_yaw)
  (bind (_direction _newtrack_0) (`Timeline|Pan` :!label _label)
    (:`Update`
      (`SceneComponent.K2_SetWorldRotation` (`self.CameraComponent`) (`KismetMathLibrary.MakeRotator` (`self.Return Value X (Roll)`) (`self.Return Value Y (Pitch)`) (+ (`self.Return Value Z (Yaw)`) _newtrack_0)) false false))
    (:`Finished`
      (`self.Reset`))))

(event `Reset`
  (`KismetSystemLibrary.Delay` 0.2)
  (`/Engine/EditorBlueprintResources/StandardMacros.FlipFlop`
    (:`A`
      (goto _label :!via `Reverse`))
    (:`B`
      (goto _label))))

(fn `UserConstructionScript`)